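; BP_Award3 is a one-time collectible pickup actor for the player character.
; On overlap with an ALS_AnimMan_CharacterBP, it activates a Niagara effect, plays audio and increments that character's AiravataCollected counter.
; An AwardCollected flag blocks repeat collection, and the actor stays in the level rather than being destroyed.
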(event `self.ReceiveActorBeginOverlap`
  (params (OtherActor :type "Actor Object Reference"))
  (if (not (`self.awardCollected`))
    (bind _asals_anim_man_character_bp (cast `/Game/AdvancedLocomotionV4/Blueprints/CharacterLogic/ALS_AnimMan_CharacterBP` OtherActor))
    (`ActorComponent.Activate` (`self.Niagara`) false)
    (`AudioComponent.Play` (`self.Audio`) 0.0)
    (set `self.awardCollected` true)
    (set `/Game/AdvancedLocomotionV4/Blueprints/CharacterLogic/ALS_AnimMan_CharacterBP.AiravataCollected` (+ (`/Game/AdvancedLocomotionV4/Blueprints/CharacterLogic/ALS_AnimMan_CharacterBP.AiravataCollected` _asals_anim_man_character_bp) 1) _asals_anim_man_character_bp)))

(fn `UserConstructionScript`)